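; Game mode that relays body-part hits on the Player and Enemy to the health bar UI.
; Every Tick it casts HealthBarWidget to HealthBar_UI and polls per-limb hit flags on both characters for head, torso, arms and legs.
; Each set flag triggers PlayHitAnimation for that side and body part, then is cleared, so the flags act as one-shot signals.
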(event EventBeginPlay)

(event EventTick
  (params (DeltaSeconds :type Float%20%28single-precision%29))
  (CallFunction|HitWidgetAnimation))

(fn ConstructionScript)

(fn HitWidgetAnimation
  (bind _player (Variables|Default|GetPlayer))
  (bind _enemy (Variables|Default|GetEnemy))
  (bind _ashealth_bar_ui (Utilities|Casting|CastToHealthBar_UI (Variables|Default|GetHealthBar_Widget)))
  (Utilities|FlowControl|Sequence
    (:then_0
      (Utilities|FlowControl|Sequence
        (:then_0
          (if (Variables|/Script/ProjectGame.FightingCharacter|GetHitHead _enemy)
            (Default|PlayHitAnimation _ashealth_bar_ui true "HitHead")
            (Variables|/Script/ProjectGame.FightingCharacter|SetHitHead _enemy false)))
        (:then_1
          (if (Variables|/Script/ProjectGame.FightingCharacter|GetHitTorso _enemy)
            (Default|PlayHitAnimation _ashealth_bar_ui true "HitTorso")
            (Variables|/Script/ProjectGame.FightingCharacter|SetHitTorso _enemy false)))
        (:then_2
          (if (Variables|/Script/ProjectGame.FightingCharacter|GetHitArmR _enemy)
            (Default|PlayHitAnimation _ashealth_bar_ui true "HitArmR")
            (Variables|/Script/ProjectGame.FightingCharacter|SetHitArmR _enemy false)))
        (:then_3
          (if (Variables|/Script/ProjectGame.FightingCharacter|GetHitArmL _enemy)
            (Default|PlayHitAnimation _ashealth_bar_ui true "HitArmL")
            (Variables|/Script/ProjectGame.FightingCharacter|SetHitArmL _enemy false)))
        (:then_4
          (if (Variables|/Script/ProjectGame.FightingCharacter|GetHitLegR _enemy)
            (Default|PlayHitAnimation _ashealth_bar_ui true "HitLegR")
            (Variables|/Script/ProjectGame.FightingCharacter|SetHitLegR _enemy false)))
        (:then_5
          (if (Variables|/Script/ProjectGame.FightingCharacter|GetHitLegL _enemy)
            (Default|PlayHitAnimation _ashealth_bar_ui true "HitLegL")
            (Variables|/Script/ProjectGame.FightingCharacter|SetHitLegL _enemy false)))))
    (:then_1
      (Utilities|FlowControl|Sequence
        (:then_0
          (if (Variables|/Script/ProjectGame.FightingCharacter|GetHitHead _player)
            (Default|PlayHitAnimation _ashealth_bar_ui false "HitHead")
            (Variables|/Script/ProjectGame.FightingCharacter|SetHitHead _player false)))
        (:then_1
          (if (Variables|/Script/ProjectGame.FightingCharacter|GetHitTorso _player)
            (Default|PlayHitAnimation _ashealth_bar_ui false "HitTorso")
            (Variables|/Script/ProjectGame.FightingCharacter|SetHitTorso _player false)))
        (:then_2
          (if (Variables|/Script/ProjectGame.FightingCharacter|GetHitArmR _player)
            (Default|PlayHitAnimation _ashealth_bar_ui false "HitArmR")
            (Variables|/Script/ProjectGame.FightingCharacter|SetHitArmR _player false)))
        (:then_3
          (if (Variables|/Script/ProjectGame.FightingCharacter|GetHitArmL _player)
            (Default|PlayHitAnimation _ashealth_bar_ui false "HitArmL")
            (Variables|/Script/ProjectGame.FightingCharacter|SetHitArmL _player false)))
        (:then_4
          (if (Variables|/Script/ProjectGame.FightingCharacter|GetHitLegR _player)
            (Default|PlayHitAnimation _ashealth_bar_ui false "HitLegR")
            (Variables|/Script/ProjectGame.FightingCharacter|SetHitLegR _player false)))
        (:then_5
          (if (Variables|/Script/ProjectGame.FightingCharacter|GetHitLegL _player)
            (Default|PlayHitAnimation _ashealth_bar_ui false "HitLegL")
            (Variables|/Script/ProjectGame.FightingCharacter|SetHitLegL _player false)))))))