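; Behavior tree task that makes an AI-controlled FightingCharacter_BP perform a random attack.
; On execute it picks one of four equally likely moves: Attack1 or Attack2, each either plain or wrapped in MoveMod.
; Each move imitates a brief button press by calling the start function, waiting a short delay, calling the matching stop, then finishing successfully.
; A failed cast stops the graph without finishing the task.
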(event EventReceiveExecuteAI
  (params (OwnerController :type AI%20Controller%20Object%20Reference) (ControlledPawn :type Pawn%20Object%20Reference))
  (bind _asfighting_character_bp (Utilities|Casting|CastToFightingCharacter_BP ControlledPawn))
  (switch int (Math|Random|RandomInteger 4)
    (:0
      (Class|FightingCharacter|Attack1 _asfighting_character_bp)
      (Utilities|FlowControl|Delay 0.1)
      (Class|FightingCharacter|StopAttack1 _asfighting_character_bp))
    (:1
      (Class|FightingCharacter|Attack2 _asfighting_character_bp)
      (Utilities|FlowControl|Delay 0.1)
      (Class|FightingCharacter|StopAttack2 _asfighting_character_bp))
    (:2
      (Class|FightingCharacter|MoveMod _asfighting_character_bp)
      (Class|FightingCharacter|Attack1 _asfighting_character_bp)
      (Utilities|FlowControl|Delay 0.1)
      (Class|FightingCharacter|StopAttack1 _asfighting_character_bp)
      (Class|FightingCharacter|StopMoveMod _asfighting_character_bp))
    (:3
      (Class|FightingCharacter|MoveMod _asfighting_character_bp)
      (Class|FightingCharacter|Attack2 _asfighting_character_bp)
      (Utilities|FlowControl|Delay 0.1)
      (Class|FightingCharacter|StopAttack2 _asfighting_character_bp)
      (Class|FightingCharacter|StopMoveMod _asfighting_character_bp)))
  (AI|BehaviorTree|FinishExecute true))