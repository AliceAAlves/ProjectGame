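; Behavior tree task that picks an AI combatant's next move: block, attack or duck.
; It selects one of two probability maps based on the TargetIsAttacking blackboard key, then compares a single random roll against the Block and Attack entries in turn.
; The entries act as cumulative thresholds, with Duck as the fallback.
; It sets exactly one of the BlockNext, AttackNext and DuckNext keys true and finishes successfully.
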(event EventReceiveExecuteAI
  (params (OwnerController :type AI%20Controller%20Object%20Reference) (ControlledPawn :type Pawn%20Object%20Reference))
  (bind _returnvalue (Utilities|Name|MakeLiteralName "DuckNext"))
  (bind _returnvalue_2 (Utilities|Name|MakeLiteralName "BlockNext"))
  (bind _returnvalue_3 (Utilities|Name|MakeLiteralName "AttackNext"))
  (bind _output_get (Variables|Default|SetBB (AI|GetBlackboard OwnerController)))
  (if (ScalableFloat|GetValueasBool _output_get (Utilities|Name|MakeLiteralName "TargetIsAttacking"))
    (Variables|Default|SetProb (Variables|Default|GetTargetIsAttackingProb))
    (else
      (Variables|Default|SetProb (Variables|Default|GetTargetIsNotAttackingProb))))
  (Variables|Default|SetRandomF (Math|Random|RandomFloat))
  (if (< (Variables|Default|GetRandomF) (.Value (Utilities|Map|Find (Variables|Default|GetProb) "Block")))
    (AI|Components|Blackboard|SetValueasBool (Variables|Default|GetBB) _returnvalue_2 true)
    (AI|Components|Blackboard|SetValueasBool (Variables|Default|GetBB) _returnvalue_3 false)
    (AI|Components|Blackboard|SetValueasBool (Variables|Default|GetBB) _returnvalue false)
    (elif (< (Variables|Default|GetRandomF) (.Value (Utilities|Map|Find (Variables|Default|GetProb) "Attack")))
      (AI|Components|Blackboard|SetValueasBool (Variables|Default|GetBB) _returnvalue_2 false)
      (AI|Components|Blackboard|SetValueasBool (Variables|Default|GetBB) _returnvalue_3 true)
      (AI|Components|Blackboard|SetValueasBool (Variables|Default|GetBB) _returnvalue false)
      (else
        (AI|Components|Blackboard|SetValueasBool (Variables|Default|GetBB) _returnvalue_2 false)
        (AI|Components|Blackboard|SetValueasBool (Variables|Default|GetBB) _returnvalue_3 false)
        (AI|Components|Blackboard|SetValueasBool (Variables|Default|GetBB) _returnvalue true))))
  (AI|BehaviorTree|FinishExecute true))